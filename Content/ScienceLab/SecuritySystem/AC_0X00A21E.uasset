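; Actor component in the ScienceLab security system that applies an "End of Transmission" screen effect to the player body's first-person camera.
; The EOT event casts the owner to BP_Body and replaces the camera's post-process settings with a single full-weight PP_EndOfTransmission1 blendable.
; BeginPlay clears DetectMode, and Tick checks that flag but performs no action.
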(event Custom|EOT
  ;[1 0 0] FatalError 0x00CE124
  (bind _asbp_body (Utilities|Casting|CastToBP_Body (Components|GetOwner)))
  (Variables|/Script/Engine.CameraComponent|SetPostProcessSettings (Variables|/Game/EurileneGene/Core/BP_Body.BP_Body_C|GetFirstPersonCamera _asbp_body) (Utilities|Struct|MakePostProcessSettings (Utilities|Struct|MakeWeightedBlendables (Utilities|Array|MakeArray (Utilities|Struct|MakeWeightedBlendable 1.0 "/Game/ScienceLab/SecuritySystem/PP_EndOfTransmission1.PP_EndOfTransmission1"))))))

(event EventBeginPlay
  ;[0 0.3281 0] Really protected, don't touch plz ! :(
  (Variables|Default|SetDetectMode false))

(event EventTick
  (params (DeltaSeconds :type Float%20%28single-precision%29))
  (if (Variables|Default|GetDetectMode)
    _))